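; BP_HW4PlayerController is a homework player controller that tests input actions and calls into the game mode and player state.
; BeginPlay casts and caches the HW4 game mode and player data state.
; Directional actions print their names, with Down also triggering the game mode's player-death call.
; Space raises HP and MP on the player state by a fixed amount and prints both.
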(event EventBeginPlay
  (Utilities|FlowControl|Sequence
    (:then_0
      (bind _asgm_hw4main_mode (Utilities|Casting|CastToGM_HW4MainMode (Game|GetGameMode)))
      (Variables|Default|SetAs%20GM%20Main%20Mode _asgm_hw4main_mode))
    (:then_1
      ;[1 1 1] PlayerState
      (bind _asps_player_data (Utilities|Casting|CastToPS_HW4PlayerData (Game|GetPlayerState 0)))
      (Variables|Default|SetAs%20PS%20Player%20Data _asps_player_data))))

(event EventTick
  (params (DeltaSeconds :type Float%20%28single-precision%29)))

(event Input|ActionEvents|InputActionmy_space
  (params (Key :type Key%20Structure))
  (:Pressed
    (Utilities|FlowControl|Sequence
      (:then_0
        (bind _output_get (Variables|/Game/HW4/PS_HW4PlayerData.PS_HW4PlayerData_C|SetPS_HP (Variables|Default|GetAs%20PS%20Player%20Data) (Math|Conversions|ToFloat(Integer) (+ 3 (Variables|/Game/HW4/PS_HW4PlayerData.PS_HW4PlayerData_C|GetPS_HP (Variables|Default|GetAs%20PS%20Player%20Data))))))
        (Development|PrintString (Utilities|String|ToString(Text) (Utilities|Text|FormatText "HP : {a}" _output_get))))
      (:then_1
        (bind _output_get_2 (Variables|/Game/HW4/PS_HW4PlayerData.PS_HW4PlayerData_C|SetPS_MP (Variables|Default|GetAs%20PS%20Player%20Data) (Math|Conversions|ToFloat(Integer) (+ 3 (Variables|/Game/HW4/PS_HW4PlayerData.PS_HW4PlayerData_C|GetPS_MP (Variables|Default|GetAs%20PS%20Player%20Data))))))
        (Development|PrintString (Utilities|String|ToString(Text) (Utilities|Text|FormatText "Mp : {a}" _output_get_2)))))))

(event Input|ActionEvents|InputActionmy_foward
  (params (Key :type Key%20Structure))
  (:Pressed
    (Development|PrintString "Foward")))

(event Input|ActionEvents|InputActionmy_left
  (params (Key :type Key%20Structure))
  (:Pressed
    (Development|PrintString "Left")))

(event Input|ActionEvents|InputActionmy_right
  (params (Key :type Key%20Structure))
  (:Pressed
    (Development|PrintString "Right")))

(event Input|ActionEvents|InputActionmy_down
  (params (Key :type Key%20Structure))
  (:Pressed
    (Development|PrintString "Down")
    (Default|CallGMPlayerDie (Variables|Default|GetAs%20GM%20Main%20Mode))))

(fn ConstructionScript)
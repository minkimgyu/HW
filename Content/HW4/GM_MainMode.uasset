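; GM_MainMode is a game mode that sets up the main UI when play begins.
; BeginPlay prints a debug greeting, then creates the WB_MainUI widget and adds it to the viewport.
; An unconnected Update chain would increment and print HP, then call MyHpUpdate once a threshold is reached, but it never runs because Tick is empty.
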(event EventBeginPlay
  (Development|PrintString "Hello")
  (bind _returnvalue (UserInterface|CreateWidget "/Game/HW4/WB_MainUI.WB_MainUI_C"))
  (UserInterface|Viewport|AddtoViewport _returnvalue 0))

(event EventTick
  (params (DeltaSeconds :type Float%20%28single-precision%29)))

(fn ConstructionScript)
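; GM_HW4MainMode is the HW4 game mode that opens the main UI and publishes chat data at BeginPlay.
; It adds WB_HW4MainUI to the viewport, then loops through DT_ChatData, relying on rows named by sequential numbers from 1.
; Each found row's name, HP, gossip and image are formatted, printed, stored in GMResult and broadcast through GMTextUpdated.
; An HP counter with a threshold-triggered MyHpUpdate call is left disconnected.
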(event EventBeginPlay
  (Utilities|FlowControl|Sequence
    (:then_0
      (bind _returnvalue (UserInterface|CreateWidget "/Game/HW4/WB_HW4MainUI.WB_HW4MainUI_C"))
      (UserInterface|Viewport|AddtoViewport _returnvalue 0))
    (:then_2
      ;[1 1 1] Get Datatable Row Count
      (bind _outrownames (DataTable|GetDataTableRowNames "/Game/HW4/DT_ChatData.DT_ChatData"))
      (Variables|Default|SetDatatable_Length (Utilities|Array|Length _outrownames))
      ;[1 1 1] Get Datatable
      (for _index (range 1 (Variables|Default|GetDatatable_Length))
        (bind _returnvalue_2 (Utilities|GetDataTableRow "/Game/HW4/DT_ChatData.DT_ChatData" (Utilities|String|StringToName (Utilities|String|ToString(Integer) _index)))
          (:then
            (Development|PrintString (Utilities|String|ToString(Text) (Utilities|Text|FormatText "Name: {1}, HP: {2}, Gossip: {3}, Image: {4}" (.Name (Utilities|Struct|BreakST_ChatData _returnvalue_2)) (.HP (Utilities|Struct|BreakST_ChatData _returnvalue_2)) (.Gossip (Utilities|Struct|BreakST_ChatData _returnvalue_2)) (.Image (Utilities|Struct|BreakST_ChatData _returnvalue_2)))))
            (bind _output_get (Variables|Default|SetGM_Result (Utilities|String|ToString(Text) (Utilities|Text|FormatText "Name: {1}, HP: {2}, Gossip: {3}, Image: {4}" (.Name (Utilities|Struct|BreakST_ChatData _returnvalue_2)) (.HP (Utilities|Struct|BreakST_ChatData _returnvalue_2)) (.Gossip (Utilities|Struct|BreakST_ChatData _returnvalue_2)) (.Image (Utilities|Struct|BreakST_ChatData _returnvalue_2))))))
            (Default|CallGMTextUpdated _output_get)))))))

(event EventTick
  (params (DeltaSeconds :type Float%20%28single-precision%29)))

(fn ConstructionScript)
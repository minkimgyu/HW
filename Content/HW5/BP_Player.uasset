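; Side-view flipbook player character that runs along the X axis and melee-attacks enemies.
; PS_PlayerData supplies attack mode, damage and the attacking flag, which blocks movement and animation updates during attacks.
; Tick watches for flipbook frame 3 to fire a DoOnce that shows the HitBox and damages overlapping BP_Enemy actors, re-armed when the animation finishes.
; Otherwise, velocity selects idle or run and flips control yaw.
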(event OnFinishedPlaying(Sprite)
  ;[1 1 1] Reset Attack
  (Sprite|SetFlipbook (Variables|Default|GetSprite) "/Game/HW5/Images/Action/Idle/_Idle1._Idle1")
  (Components|Timeline|SetLooping (Variables|Default|GetSprite) true)
  (if (not (Audio|Components|Audio|IsPlaying (Variables|Default|GetSprite)))
    (Audio|Components|Audio|Play (Variables|Default|GetSprite))
    (Variables|/Game/HW5/PS_PlayerData.PS_PlayerData_C|SetIsAttacking (Variables|Default|GetAs%20PS%20HW5Player%20Data) false)
    (CallFunction|ResetAttack)
    (Development|SetHiddeninGame (Variables|Default|GetHitBox) true false)))

(event Custom|Hit
  ;[1 1 1] Hit
  (for _array_element (Collision|GetOverlappingActors (Variables|Default|GetHitBox) "/Game/HW5/BP_Enemy.BP_Enemy_C" :!class /Script/Engine.PrimitiveComponent)
    (Game|Damage|ApplyDamage _array_element (Variables|/Game/HW5/PS_PlayerData.PS_PlayerData_C|GetPlayerDamage (Variables|Default|GetAs%20PS%20HW5Player%20Data)) 0 0)))

(event Custom|ResetAttack
  ;[1 1 1] Check Hit Frame
  (Utilities|FlowControl|DoOnce false) ; enters at Reset
)

(event Custom|UpdateAnimation
  ;[1 1 1] Play Run Animation
  (Sprite|SetFlipbook (Variables|Default|GetSprite) (select (> (Math|Vector|VectorLength (Variables|/Script/Engine.MovementComponent|GetVelocity (Variables|Character|GetCharacterMovement))) 0.0) "/Game/HW5/Images/Action/Run/_Run1._Run1" "/Game/HW5/Images/Action/Idle/_Idle1._Idle1")))

(event Custom|UpdateControlRotation
  ;[1 1 1] PlayerFlip
  (Utilities|IsValid (Pawn|GetController)
    (:Is%20Valid
      (Math|Float|CompareFloat (.X (Math|Vector|BreakVector (Variables|/Script/Engine.MovementComponent|GetVelocity (Variables|Character|GetCharacterMovement)))) 0.0
        (:>
          (Pawn|SetControlRotation (Pawn|GetController) (Math|Rotator|MakeRotator 0.0 0.0 0.0)))
        (:<
          (Pawn|SetControlRotation (Pawn|GetController) (Math|Rotator|MakeRotator 0.0 0.0 1.8e+02)))))))

(event Custom|Move
  (params (AxisValue :type Float%20%28double-precision%29))
  ;[1 1 1] Move
  (if (not (Variables|/Game/HW5/PS_PlayerData.PS_PlayerData_C|GetIsAttacking (Variables|Default|GetAs%20PS%20HW5Player%20Data)))
    (Pawn|Input|AddMovementInput "1.000000,0.000000,0.000000" AxisValue false)))

(event Custom|Attack
  ;[1 1 1] Attack
  (switch int (- (Variables|/Game/HW5/PS_PlayerData.PS_PlayerData_C|GetPlayerAttackMode (Variables|Default|GetAs%20PS%20HW5Player%20Data)) 1)
    (:0
      (Sprite|SetFlipbook (Variables|Default|GetSprite) "/Game/HW5/Images/Action/Attack/Attack1/_Attack1._Attack1"))
    (:1
      (Sprite|SetFlipbook (Variables|Default|GetSprite) "/Game/HW5/Images/Action/Attack/Attack2/_Attack3._Attack3")))
  (Components|Timeline|SetLooping (Variables|Default|GetSprite) false)
  (Variables|/Game/HW5/PS_PlayerData.PS_PlayerData_C|SetIsAttacking (Variables|Default|GetAs%20PS%20HW5Player%20Data) true))

(event EventBeginPlay
  ;[1 1 1] Cast PlayerData
  (bind _asps_hw5player_data (Utilities|Casting|CastToPS_PlayerData (Game|GetPlayerState 0)))
  (Variables|Default|SetAs%20PS%20HW5Player%20Data _asps_hw5player_data))

(event EventTick
  (params (DeltaSeconds :type Float%20%28single-precision%29))
  ;[1 1 1] Check Hit Frame
  (Utilities|FlowControl|Sequence
    (:then_0
      (if (Variables|/Game/HW5/PS_PlayerData.PS_PlayerData_C|GetIsAttacking (Variables|Default|GetAs%20PS%20HW5Player%20Data))
        (if (== (Class|PaperFlipbookComponent|GetPlaybackPositioninFrames (Variables|Default|GetSprite)) 3)
          (Utilities|FlowControl|DoOnce false
            (:Completed
              (CallFunction|Hit)
              (Development|SetHiddeninGame (Variables|Default|GetHitBox) false false)))
          (else
            (Development|SetHiddeninGame (Variables|Default|GetHitBox) true false)))))
    (:then_1
      (if (not (Variables|/Game/HW5/PS_PlayerData.PS_PlayerData_C|GetIsAttacking (Variables|Default|GetAs%20PS%20HW5Player%20Data)))
        (CallFunction|UpdateAnimation)
        (CallFunction|UpdateControlRotation)))))

(fn ConstructionScript)
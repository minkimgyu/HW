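; GM_HW5MainMode is the game mode for HW5, creating the main HUD widget and managing enemy health and player attack mode.
; All values live in PS_HW5PlayerData, cached from player state 0 at BeginPlay.
; Heal and damage events clamp enemy HP, toggle death and revive, and attack mode cycles back to 1 past its maximum.
; Each change fires a Call event, such as CallEnemyHpUpdate or CallEnemyDie, to signal the result.
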(event Custom|HealToEnemy
  (bind _as_ps_hw5player_data (Variables|Default|GetAs%20PS%20HW5Player%20Data))
  (if (Variables|/Game/HW5/PS_HW5PlayerData.PS_HW5PlayerData_C|GetEnemyDie (Variables|Default|GetAs%20PS%20HW5Player%20Data))
    (CallFunction|Revive)
    (Default|CallEnemyRevive))
  (if (<= (+ (Variables|/Game/HW5/PS_HW5PlayerData.PS_HW5PlayerData_C|GetEnemyHp (Variables|Default|GetAs%20PS%20HW5Player%20Data)) (Variables|/Game/HW5/PS_HW5PlayerData.PS_HW5PlayerData_C|GetEnemyHealPoint (Variables|Default|GetAs%20PS%20HW5Player%20Data))) (Variables|/Game/HW5/PS_HW5PlayerData.PS_HW5PlayerData_C|GetEnemyOriginHp (Variables|Default|GetAs%20PS%20HW5Player%20Data)))
    (Variables|/Game/HW5/PS_HW5PlayerData.PS_HW5PlayerData_C|SetEnemyHp _as_ps_hw5player_data (+ (Variables|/Game/HW5/PS_HW5PlayerData.PS_HW5PlayerData_C|GetEnemyHp (Variables|Default|GetAs%20PS%20HW5Player%20Data)) (Variables|/Game/HW5/PS_HW5PlayerData.PS_HW5PlayerData_C|GetEnemyHealPoint (Variables|Default|GetAs%20PS%20HW5Player%20Data))))
    (else
      (Variables|/Game/HW5/PS_HW5PlayerData.PS_HW5PlayerData_C|SetEnemyHp _as_ps_hw5player_data (Variables|/Game/HW5/PS_HW5PlayerData.PS_HW5PlayerData_C|GetEnemyOriginHp (Variables|Default|GetAs%20PS%20HW5Player%20Data)))))
  (Default|CallEnemyHpUpdate))

(event Custom|DamageToEnemy
  (params (damage :type Float%20%28double-precision%29))
  (if (<= (- (Variables|/Game/HW5/PS_HW5PlayerData.PS_HW5PlayerData_C|GetEnemyHp (Variables|Default|GetAs%20PS%20HW5Player%20Data)) damage) 0.0)
    (Variables|/Game/HW5/PS_HW5PlayerData.PS_HW5PlayerData_C|SetEnemyHp (Variables|Default|GetAs%20PS%20HW5Player%20Data) 0.0)
    (Variables|/Game/HW5/PS_HW5PlayerData.PS_HW5PlayerData_C|SetEnemyDie (Variables|Default|GetAs%20PS%20HW5Player%20Data) true)
    (Default|CallEnemyDie)
    (else
      (Variables|/Game/HW5/PS_HW5PlayerData.PS_HW5PlayerData_C|SetEnemyHp (Variables|Default|GetAs%20PS%20HW5Player%20Data) (- (Variables|/Game/HW5/PS_HW5PlayerData.PS_HW5PlayerData_C|GetEnemyHp (Variables|Default|GetAs%20PS%20HW5Player%20Data)) damage))))
  (Default|CallEnemyHpUpdate))

(event Custom|ChangeAttackMode
  (if (> (+ (Variables|/Game/HW5/PS_HW5PlayerData.PS_HW5PlayerData_C|GetPlayerAttackMode (Variables|Default|GetAs%20PS%20HW5Player%20Data)) 1) (Variables|/Game/HW5/PS_HW5PlayerData.PS_HW5PlayerData_C|GetPlayerMaxAttackMode (Variables|Default|GetAs%20PS%20HW5Player%20Data)))
    (Variables|/Game/HW5/PS_HW5PlayerData.PS_HW5PlayerData_C|SetPlayerAttackMode (Variables|Default|GetAs%20PS%20HW5Player%20Data) 1)
    (else
      (Variables|/Game/HW5/PS_HW5PlayerData.PS_HW5PlayerData_C|SetPlayerAttackMode (Variables|Default|GetAs%20PS%20HW5Player%20Data) (+ (Variables|/Game/HW5/PS_HW5PlayerData.PS_HW5PlayerData_C|GetPlayerAttackMode (Variables|Default|GetAs%20PS%20HW5Player%20Data)) 1))))
  (Default|CallPlayerAttackModeUpdate))

(event Custom|Revive
  (Variables|/Game/HW5/PS_HW5PlayerData.PS_HW5PlayerData_C|SetEnemyDie (Variables|Default|GetAs%20PS%20HW5Player%20Data) false))

(event EventBeginPlay
  (Utilities|FlowControl|Sequence
    (:then_0
      (bind _returnvalue (UserInterface|CreateWidget "/Game/HW5/WB_HW5MainUI.WB_HW5MainUI_C"))
      (UserInterface|Viewport|AddtoViewport _returnvalue 0))
    (:then_1
      (bind _asps_hw5player_data (Utilities|Casting|CastToPS_HW5PlayerData (Game|GetPlayerState 0)))
      (Variables|Default|SetAs%20PS%20HW5Player%20Data _asps_hw5player_data))))

(fn ConstructionScript)
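; BP_HW5Enemy is a flipbook-sprite enemy that forwards any damage it takes to GM_HW5MainMode.
; On BeginPlay it caches the game mode and binds its Die and Revive events to the mode's enemy die and revive events.
; Die switches the sprite to a non-looping death flipbook, and Revive restores the looping idle one, restarting playback if it stopped.
; The enemy keeps no health state of its own.
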(event Custom|Die
  (Sprite|SetFlipbook (Variables|Default|GetSprite) "/Game/HW5/Images/Action/Death/_Death1._Death1")
  (Components|Timeline|SetLooping (Variables|Default|GetSprite) false))

(event Custom|Revive
  (Sprite|SetFlipbook (Variables|Default|GetSprite) "/Game/HW5/Images/Action/Idle/_Idle1._Idle1")
  (Components|Timeline|SetLooping (Variables|Default|GetSprite) true)
  (if (not (Audio|Components|Audio|IsPlaying (Variables|Default|GetSprite)))
    (Audio|Components|Audio|Play (Variables|Default|GetSprite))))

(event EventBeginPlay
  (Utilities|FlowControl|Sequence
    (:then_0
      (bind _asgm_hw5main_mode (Utilities|Casting|CastToGM_HW5MainMode (Game|GetGameMode)))
      (Variables|Default|SetAs%20GM%20HW5Main%20Mode _asgm_hw5main_mode))
    (:then_1
      (EventDispatchers|BindEventtoEnemyDie (Variables|Default|GetAs%20GM%20HW5Main%20Mode) (delegate Custom|Die)))
    (:then_2
      (EventDispatchers|BindEventtoEnemyRevive (Variables|Default|GetAs%20GM%20HW5Main%20Mode) (delegate Custom|Revive)))))

(event Collision|EventActorBeginOverlap
  (params (OtherActor :type Actor%20Object%20Reference)))

(event EventTick
  (params (DeltaSeconds :type Float%20%28single-precision%29)))

(event Game|Damage|EventAnyDamage
  (params (Damage :type Float%20%28single-precision%29) (DamageType :type Damage%20Type%20Object%20Reference) (InstigatedBy :type Controller%20Object%20Reference) (DamageCauser :type Actor%20Object%20Reference))
  (Default|DamagetoEnemy (Variables|Default|GetAs%20GM%20HW5Main%20Mode) Damage))

(fn ConstructionScript)